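; BP_KCBase is a character Blueprint that carries a sword and provides a montage-driven melee attack.
; On BeginPlay it spawns BP_BasicSword, snaps it to the mesh's Sword socket and stores it as Weapon.
; TryMelee starts the melee montage or, if it is already in its first attack section, queues the second as a combo.
; TryMagic is an empty stub.
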(event `CreateSword`
  (bind _returnvalue (`|SpawnActorFromClass` "/Game/Blueprints/BP_BasicSword.BP_BasicSword_C" (`self.GetTransform`) "Undefined" "OverrideRootScale"))
  (`self.K2_AttachToComponent` _returnvalue (`self.Mesh`) "Sword" "SnapToTarget" "SnapToTarget" "SnapToTarget" false)
  (set `self.Weapon` _returnvalue))

(event `self.ReceiveBeginPlay`
  (`self.CreateSword`))

(event `TryMelee`
  (bind _returnvalue (`SkeletalMeshComponent.GetAnimInstance` (`self.Mesh`)))
  (bind _returnvalue_2 (`AnimInstance.Montage_GetCurrentSection` _returnvalue "/Game/Assets/Knight/Animations/AN_MeleeAttack.AN_MeleeAttack"))
  (if (`AnimInstance.Montage_IsActive` _returnvalue "/Game/Assets/Knight/Animations/AN_MeleeAttack.AN_MeleeAttack")
    (switch `name` _returnvalue_2
      (:`Attack1`
        (`AnimInstance.Montage_SetNextSection` _returnvalue _returnvalue_2 "Attack2" null)))
    (else
      (`self.PlayAnimMontage` "/Game/Assets/Knight/Animations/AN_MeleeAttack.AN_MeleeAttack" 1.0 "Attack1"))))

(event `TryMagic`)

(fn `UserConstructionScript`)